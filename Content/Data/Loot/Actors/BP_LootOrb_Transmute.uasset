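; BP_LootOrb_Transmute is a currency loot orb that launches when spawned and is collected by the first-person character on overlap.
; On BeginPlay, OrbMesh receives a velocity-change impulse in a random, upward-biased direction with extra vertical force.
; A delay then enables pickup, and later PickupSphere begin-overlaps grant the configured currency type and amount before destroying the orb.
; Overlaps that begin during the delay are ignored.
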(event `self.ReceiveBeginPlay`
  (`PrimitiveComponent.AddImpulse` (`self.OrbMesh`) (+ (* (`KismetMathLibrary.Normal` (`KismetMathLibrary.MakeVector` (.x (`KismetMathLibrary.RandomUnitVector`)) (.y (`KismetMathLibrary.RandomUnitVector`)) (+ (`self.UpdwardBias`) (`KismetMathLibrary.Abs` (.z (`KismetMathLibrary.RandomUnitVector`)))))) (`self.LaunchStrength`)) (`KismetMathLibrary.MakeVector` 0.0 0.0 (`self.ExtraUpwardForce`))) "None" true)
  (`KismetSystemLibrary.Delay` (`self.PickupDelay`))
  (set `self.bCanPickup` true))

(event `self.PickupSphere.OnComponentBeginOverlap`
  (params (OverlappedComponent :type "PrimitiveComponent Object Reference") (OtherActor :type "Actor Object Reference") (OtherComp :type "PrimitiveComponent Object Reference") (OtherBodyIndex :type Integer) (bFromSweep :type Boolean) (SweepResult :type "HitResult Structure (by ref)"))
  (if (`self.bCanPickup`)
    (bind _asbp_first_person_character (cast `/Game/FirstPerson/Blueprints/BP_FirstPersonCharacter` OtherActor))
    (`/Game/FirstPerson/Blueprints/BP_FirstPersonCharacter.AddCurrency` _asbp_first_person_character (`self.CurrencyType`) (`self.Amount`))
    (`self.K2_DestroyActor`)))

(fn `UserConstructionScript`)