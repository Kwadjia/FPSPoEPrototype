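; BP_EnemyFlying is an enemy character that chases the first-person player and can be killed by damage.
; A looping timer, rather than Tick, runs UpdateAggroMove, which latches aggro once the player is within range and issues AI MoveToActor orders.
; AnyDamage reduces health and calls Die, which stops movement, disables capsule collision and sets a short lifespan.
; GetDamageMultiplier is an unfinished hit-component comparison, and no flight-specific logic appears.
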(event `self.ReceiveBeginPlay`
  (`KismetSystemLibrary.PrintString` "Enemy Begin Play")
  (set `self.Health` (`self.MaxHealth`))
  (set `self.bIsDead` false)
  (bind _asbp_first_person_character (cast `/Game/FirstPerson/Blueprints/BP_FirstPersonCharacter` (`GameplayStatics.GetPlayerCharacter` 0))
    (:`then`
      (set `self.PlayerRef` _asbp_first_person_character)
      (`KismetSystemLibrary.K2_SetTimer` null "UpdateAggroMove" (`self.MoveUpdateInterval`) true true))
    (:`CastFailed`
      (`KismetSystemLibrary.PrintString` "Cast Failed"))))

(event `self.ReceiveAnyDamage`
  (params (Damage :type "Float (single-precision)") (DamageType :type "DamageType Object Reference") (InstigatedBy :type "Controller Object Reference") (DamageCauser :type "Actor Object Reference"))
  (if (not (`self.bIsDead`))
    (bind _output_get (set `self.Health` (- (`self.Health`) Damage)))
    (if (<= _output_get 0.0)
      (set `self.bIsDead` true)
      (`self.Die`))))

(fn `Die`
  (`MovementComponent.StopMovementImmediately` (`self.CharacterMovement`))
  (`PrimitiveComponent.SetCollisionEnabled` (`self.CapsuleComponent`) "NoCollision")
  (`PrimitiveComponent.SetSimulatePhysics` (`self.VisualMesh`) false)
  (`self.SetLifeSpan` 1.5)
  (`KismetSystemLibrary.PrintString` "Target Destroyed"))

(fn `GetDamageMultiplier`
  (params (HitComponent :type "PrimitiveComponent Object Reference"))
  (returns (bIsWeakPoint :type Boolean))
  (return (== HitComponent null)))

(fn `UpdateAggroMove`
  (bind _returnvalue (`GameplayStatics.GetPlayerCharacter` 0))
  (bind _returnvalue_2 (`self.GetController`))
  (if (not (`self.bIsDead`))
    (bind _asbp_first_person_character (cast `/Game/FirstPerson/Blueprints/BP_FirstPersonCharacter` _returnvalue))
    (bind _output_get (set `self.PlayerRef` _asbp_first_person_character))
    (if (`KismetSystemLibrary.IsValid` _output_get)
      (if (`self.bIsAggro`)
        (bind _asaicontroller (cast `AIController` _returnvalue_2 :!label _label))
        (`AIController.MoveToActor` _asaicontroller _returnvalue 100.0 true true true null true)
        (elif (<= (`KismetMathLibrary.Vector_Distance` (`self.K2_GetActorLocation`) (`self.K2_GetActorLocation` _output_get)) (`self.AggroRange`))
          (set `self.bIsAggro` true)
          (goto _label)
          (else
            (`Controller.StopMovement` _returnvalue_2)))))))

(fn `UserConstructionScript`)